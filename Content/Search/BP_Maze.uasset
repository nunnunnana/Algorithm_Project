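; Maze actor that spawns a grid of random walls and open points between corner start and end points, for visualizing pathfinding searches.
; StartDFS takes random unchecked neighbors with a short delay, backtracks on a stack, colors visited stack cells green on success and reports reached or unreached.
; StartBFS floods outward from a timer-driven queue without an end-point check.
; Both find neighbors by comparing every cell's location; the gradual-recolor timers are unused.
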(event `self.ReceiveBeginPlay`
  ;[1 1 1] 미로 생성
  (for _index (range (+ (`self.height`) 1)) :!label _label
    (for _index_2 (range (+ (`self.width`) 1))
      (if (and (== _index_2 (`self.width`)) (== _index (`self.height`)))
        (bind _returnvalue (`KismetMathLibrary.Conv_IntToDouble` (* _index 100)))
        (bind _returnvalue_2 (`KismetMathLibrary.Conv_IntToDouble` (* _index_2 100)))
        (bind _returnvalue_3 (`|SpawnActorFromClass` "/Game/Search/BP_EndPoint.BP_EndPoint_C" (`KismetMathLibrary.MakeTransform` (`KismetMathLibrary.MakeVector` _returnvalue _returnvalue_2 25.0) (struct) (0.5 0.5 0.5)) "Undefined" "MultiplyWithRoot" null null))
        (`KismetArrayLibrary.Array_Add` (`self.graphActor`) _returnvalue_3)
        (elif (and (== _index_2 0) (== _index 0))
          (bind _returnvalue_4 (`|SpawnActorFromClass` "/Game/Search/BP_StartPoint.BP_StartPoint_C" (`KismetMathLibrary.MakeTransform` (`KismetMathLibrary.MakeVector` _returnvalue _returnvalue_2 25.0) (struct) (0.5 0.5 0.5)) "Undefined" "MultiplyWithRoot" null null))
          (set `self.StartPoint` _returnvalue_4)
          (elif (!= (`KismetMathLibrary.RandomIntegerInRange` 0 (`self.Distribution `)) 0)
            (bind _returnvalue_5 (`|SpawnActorFromClass` "/Game/Search/BP_Points.BP_Points_C" (`KismetMathLibrary.MakeTransform` (`KismetMathLibrary.MakeVector` _returnvalue _returnvalue_2 25.0) (struct) (0.5 0.5 0.5)) "Undefined" "MultiplyWithRoot" null null))
            (`KismetArrayLibrary.Array_Add` (`self.graphActor`) _returnvalue_5)
            (else
              (bind _returnvalue_6 (`|SpawnActorFromClass` "/Game/Search/BP_Wall.BP_Wall_C" (`KismetMathLibrary.MakeTransform` (`KismetMathLibrary.MakeVector` _returnvalue _returnvalue_2 25.0) (struct) (0.5 0.5 0.5)) "Undefined" "MultiplyWithRoot" null null))
              (`KismetArrayLibrary.Array_Add` (`self.graphActor`) _returnvalue_6))))))))

(event `DrawMap`
  ;[1 1 1] 미로 생성
  (goto _label))

(event `ResetMap`
  ;[1 1 1] 초기화
  (`|ExecutionSequence`
    (:`then_0`
      (bind _outactors (`GameplayStatics.GetAllActorsOfClass` "/Game/Search/BP_Points.BP_Points_C"))
      (`self.K2_DestroyActor` _outactors))
    (:`then_1`
      (set `self.IsFindEndPoint` false)
      (`KismetArrayLibrary.Array_Clear` (`self.ArrCurrentCell`))
      (`KismetArrayLibrary.Array_Clear` (`self.graphActor`))
      (`self.DrawMap`))))

(event `StartDFS`
  (params (CurrentCell :type "/Game/Search/BP_Points Object Reference"))
  (bind _returnvalue (`KismetArrayLibrary.Array_Length` (`self.CellArray`)))
  (bind (_returnvalue_x _returnvalue_y) (`KismetMathLibrary.BreakVector` (`self.K2_GetActorLocation` (`self.CurrentCell`))))
  (bind (_returnvalue_x_2 _returnvalue_y_2) (`KismetMathLibrary.BreakVector` (`self.K2_GetActorLocation` (`self.CurrentCell`))))
  (bind (_returnvalue_x_3 _returnvalue_y_3) (`KismetMathLibrary.BreakVector` (`self.K2_GetActorLocation` (`self.CurrentCell`))))
  (bind (_returnvalue_x_4 _returnvalue_y_4) (`KismetMathLibrary.BreakVector` (`self.K2_GetActorLocation` (`self.CurrentCell`))))
  (bind _output (`|GetArrayItem` (`self.ArrCurrentCell`) (`KismetArrayLibrary.Array_LastIndex` (`self.ArrCurrentCell`))))
  ;[1 1 1] DFS
  ;;[1 1 1] 기준이 되는 point 설정
  (`/Engine/EditorBlueprintResources/StandardMacros.IsValid` CurrentCell
    (:`Is Valid`
      (set `self.CurrentCell` CurrentCell))
    (:`Is Not Valid`
      (set `self.CurrentCell` (`self.StartPoint`))))
  (`KismetArrayLibrary.Array_Clear` (`self.CellArray`))
  (for _array_element (`self.graphActor`)
    (if (not (`/Game/Search/BP_Points.IsChecked` _array_element))
      (bind (_returnvalue_x_5 _returnvalue_y_5) (`KismetMathLibrary.BreakVector` (`self.K2_GetActorLocation` _array_element)))
      ;;[1 1 1] 왼쪽 확인
      (if (and (== _returnvalue_x_5 (- _returnvalue_x 100.0)) (== _returnvalue_y_5 _returnvalue_y))
        (`KismetArrayLibrary.Array_Add` (`self.CellArray`) _array_element))
      (bind (_returnvalue_x_6 _returnvalue_y_6) (`KismetMathLibrary.BreakVector` (`self.K2_GetActorLocation` _array_element)))
      ;;[1 1 1] 오른쪽 확인
      (if (and (== _returnvalue_x_6 (+ _returnvalue_x_2 100.0)) (== _returnvalue_y_6 _returnvalue_y_2))
        (`KismetArrayLibrary.Array_Add` (`self.CellArray`) _array_element))
      (bind (_returnvalue_x_7 _returnvalue_y_7) (`KismetMathLibrary.BreakVector` (`self.K2_GetActorLocation` _array_element)))
      ;;[1 1 1] 위쪽 확인
      (if (and (== _returnvalue_y_7 (+ _returnvalue_y_3 100.0)) (== _returnvalue_x_7 _returnvalue_x_3))
        (`KismetArrayLibrary.Array_Add` (`self.CellArray`) _array_element))
      (bind (_returnvalue_x_8 _returnvalue_y_8) (`KismetMathLibrary.BreakVector` (`self.K2_GetActorLocation` _array_element)))
      ;;[1 1 1] 위쪽 확인
      (if (and (== _returnvalue_y_8 (- _returnvalue_y_4 100.0)) (== _returnvalue_x_8 _returnvalue_x_4))
        (`KismetArrayLibrary.Array_Add` (`self.CellArray`) _array_element))))
  ;;[1 1 1] CellArray에 End point 있는지 확인
  (for _array_element_2 (`self.CellArray`)
    (if (`/Game/Search/BP_Points.IsEndPoint` _array_element_2)
      (set `self.IsFindEndPoint` true)
      (else
        (`KismetArrayLibrary.Array_Add` (`self.ArrCurrentCell`) _array_element_2))))
  ;;[1 1 1] 방문했던 Cell의 색상 변경
  (if (`self.IsFindEndPoint`)
    (for _array_element_3 (`self.ArrCurrentCell`)
      (if (`/Game/Search/BP_Points.IsVisited` _array_element_3)
        (`/Game/Search/BP_Points.SetMaterial` _array_element_3 "/Game/Asset/Material/M_Base_Green.M_Base_Green")))
    (`self.DestinationReached`)
    (else
      ;;[1 1 1] 상하좌우 중 Cell이 있으면 랜덤으로 하나 정해서 Next Cell 설정 후 색상 변경
      ;; 만약 Cell 이 없으면 ArrCurrentCell 마지막 인덱스 -1 을 Next Cell 로 설정 후 함수 호출
      (if (== _returnvalue 0)
        (`KismetArrayLibrary.Array_Remove` (`self.ArrCurrentCell`) (`KismetArrayLibrary.Array_LastIndex` (`self.ArrCurrentCell`)))
        (`/Engine/EditorBlueprintResources/StandardMacros.IsValid` _output
          (:`Is Valid`
            (bind _output_get (set `self.NextCell` _output))
            (`/Game/Search/BP_Points.SetVisited` _output_get)
            (`self.StartDFS` (`self.NextCell`)))
          (:`Is Not Valid`
            (`self.DestinationUnreached`)))
        (else
          (bind _output_get_2 (set `self.NextCell` (`|GetArrayItem` (`self.CellArray`) (`KismetMathLibrary.RandomInteger` _returnvalue))))
          (`/Game/Search/BP_Points.SetVisited` _output_get_2)
          (`KismetSystemLibrary.Delay` 0.1)
          (`self.StartDFS` (`self.NextCell`)))))))

(event `ActivateVisitedCell`
  (bind _output (`|GetArrayItem` (`self.ArrCurrentCell`) (- (`self.arrCurrentLengh`) 1)))
  ;[1 1 1] DFS
  ;;[1 0 0] 서서히 변하도록 타이머 사용 (미사용)
  (if (<= (`self.arrCurrentLengh`) 0)
    (`KismetSystemLibrary.K2_ClearAndInvalidateTimerHandle` (`self.DFSTimer`))
    (`self.DestinationReached`)
    (else
      (if (`/Game/Search/BP_Points.IsVisited` _output)
        (`/Game/Search/BP_Points.SetChangeColor` _output))
      (`/Engine/EditorBlueprintResources/StandardMacros.DecrementInt` (`self.arrCurrentLengh`)))))

(event `StartBFS`
  ;[1 1 1] BFS
  ;;[1 1 1] 기준이 되는 point 설정
  (set `self.CurrentCell` (`self.StartPoint`))
  (`KismetArrayLibrary.Array_Clear` (`self.CellArray`))
  (`KismetArrayLibrary.Array_Add` (`self.ArrCurrentCell`) (`self.CurrentCell`))
  (bind _returnvalue (`KismetSystemLibrary.K2_SetTimerDelegate` (delegate `CustomEvent`) 0.2 true)))

(event `CustomEvent`
  (bind (_returnvalue_x _returnvalue_y) (`KismetMathLibrary.BreakVector` (`self.K2_GetActorLocation` (`self.CurrentCell`))))
  (bind (_returnvalue_x_2 _returnvalue_y_2) (`KismetMathLibrary.BreakVector` (`self.K2_GetActorLocation` (`self.CurrentCell`))))
  (bind (_returnvalue_x_3 _returnvalue_y_3) (`KismetMathLibrary.BreakVector` (`self.K2_GetActorLocation` (`self.CurrentCell`))))
  (bind (_returnvalue_x_4 _returnvalue_y_4) (`KismetMathLibrary.BreakVector` (`self.K2_GetActorLocation` (`self.CurrentCell`))))
  ;[1 1 1] BFS
  (if (not (`KismetArrayLibrary.Array_IsEmpty` (`self.ArrCurrentCell`)))
    (set `self.CurrentCell` (`|GetArrayItem` (`self.ArrCurrentCell`)))
    (`KismetArrayLibrary.Array_Remove` (`self.ArrCurrentCell`))
    (for _array_element (`self.graphActor`)
      (if (not (`/Game/Search/BP_Points.IsChecked` _array_element))
        (bind (_returnvalue_x_5 _returnvalue_y_5) (`KismetMathLibrary.BreakVector` (`self.K2_GetActorLocation` _array_element)))
        ;;[1 1 1] 왼쪽 확인
        (if (and (== _returnvalue_x_5 (- _returnvalue_x_2 100.0)) (== _returnvalue_y_5 _returnvalue_y_2))
          (`KismetArrayLibrary.Array_Add` (`self.CellArray`) _array_element))
        (bind (_returnvalue_x_6 _returnvalue_y_6) (`KismetMathLibrary.BreakVector` (`self.K2_GetActorLocation` _array_element)))
        ;;[1 1 1] 오른쪽 확인
        (if (and (== _returnvalue_x_6 (+ _returnvalue_x_3 100.0)) (== _returnvalue_y_6 _returnvalue_y_3))
          (`KismetArrayLibrary.Array_Add` (`self.CellArray`) _array_element))
        (bind (_returnvalue_x_7 _returnvalue_y_7) (`KismetMathLibrary.BreakVector` (`self.K2_GetActorLocation` _array_element)))
        ;;[1 1 1] 위쪽 확인
        (if (and (== _returnvalue_y_7 (+ _returnvalue_y_4 100.0)) (== _returnvalue_x_7 _returnvalue_x_4))
          (`KismetArrayLibrary.Array_Add` (`self.CellArray`) _array_element))
        (bind (_returnvalue_x_8 _returnvalue_y_8) (`KismetMathLibrary.BreakVector` (`self.K2_GetActorLocation` _array_element)))
        ;;[1 1 1] 위쪽 확인
        (if (and (== _returnvalue_y_8 (- _returnvalue_y 100.0)) (== _returnvalue_x_8 _returnvalue_x))
          (`KismetArrayLibrary.Array_Add` (`self.CellArray`) _array_element))))
    ;;[1 1 1] CellArray에 End point 있는지 확인
    (for _array_element_2 (`self.CellArray`)
      (`/Game/Search/BP_Points.SetVisited` _array_element_2)
      (`KismetArrayLibrary.Array_Add` (`self.ArrCurrentCell`) _array_element_2))
    (`KismetArrayLibrary.Array_Clear` (`self.CellArray`))
    (else
      (`KismetSystemLibrary.K2_ClearAndInvalidateTimerHandle` (stale `StartBFS` _returnvalue))
      (`KismetSystemLibrary.PrintString` "Hello"))))

(event `CustomEvent_1`
  (bind _output (`|GetArrayItem` (`self.ArrCurrentCell`) (- (`self.arrCurrentLengh`) 1)))
  ;[1 1 1] BFS
  ;;[1 0 0] 서서히 변하도록 타이머 사용 (미사용)
  (if (<= (`self.arrCurrentLengh`) 0)
    (`KismetSystemLibrary.K2_ClearAndInvalidateTimerHandle` (`self.DFSTimer`))
    (`self.DestinationReached`)
    (else
      (if (`/Game/Search/BP_Points.IsVisited` _output)
        (`/Game/Search/BP_Points.SetChangeColor` _output))
      (`/Engine/EditorBlueprintResources/StandardMacros.DecrementInt` (`self.arrCurrentLengh`)))))

(fn `UserConstructionScript`)
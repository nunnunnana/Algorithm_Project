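; Pathfinding visualizer that spawns a random grid maze of walls, points, start and end, then runs DFS, BFS or Dijkstra on it.
; Neighbors come from scanning all spawned cells for adjacent locations.
; DFS recurses randomly with backtracking, BFS drains a timer-driven queue, and both turn visited cells green on success.
; Dijkstra expands delayed uniform-cost waves, then traces decreasing costs back from the end to color the path.
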(event `self.ReceiveBeginPlay`
  ;[1 1 1] 미로 생성
  (for _index (range (+ (`self.height`) 1)) :!label _label
    (for _index_2 (range (+ (`self.width`) 1))
      (if (and (== _index_2 (`self.width`)) (== _index (`self.height`)))
        (bind _returnvalue (`KismetMathLibrary.Conv_IntToDouble` (* _index 100)))
        (bind _returnvalue_2 (`KismetMathLibrary.Conv_IntToDouble` (* _index_2 100)))
        (bind _returnvalue_3 (`|SpawnActorFromClass` "/Game/Search/BP_EndPoint.BP_EndPoint_C" (`KismetMathLibrary.MakeTransform` (`KismetMathLibrary.MakeVector` _returnvalue _returnvalue_2 25.0) (struct) (0.5 0.5 0.5)) "Undefined" "MultiplyWithRoot" null null))
        (`KismetArrayLibrary.Array_Add` (`self.graphActor`) _returnvalue_3)
        (elif (and (== _index_2 0) (== _index 0))
          (bind _returnvalue_4 (`|SpawnActorFromClass` "/Game/Search/BP_StartPoint.BP_StartPoint_C" (`KismetMathLibrary.MakeTransform` (`KismetMathLibrary.MakeVector` _returnvalue _returnvalue_2 25.0) (struct) (0.5 0.5 0.5)) "Undefined" "MultiplyWithRoot" null null))
          (set `self.StartPoint` _returnvalue_4)
          (elif (!= (`KismetMathLibrary.RandomIntegerInRange` 0 (`self.Distribution `)) 0)
            (bind _returnvalue_5 (`|SpawnActorFromClass` "/Game/Search/BP_Points.BP_Points_C" (`KismetMathLibrary.MakeTransform` (`KismetMathLibrary.MakeVector` _returnvalue _returnvalue_2 25.0) (struct) (0.5 0.5 0.5)) "Undefined" "MultiplyWithRoot" null null))
            (`KismetArrayLibrary.Array_Add` (`self.graphActor`) _returnvalue_5)
            (else
              (bind _returnvalue_6 (`|SpawnActorFromClass` "/Game/Search/BP_Wall.BP_Wall_C" (`KismetMathLibrary.MakeTransform` (`KismetMathLibrary.MakeVector` _returnvalue _returnvalue_2 25.0) (struct) (0.5 0.5 0.5)) "Undefined" "MultiplyWithRoot" null null))
              (`KismetArrayLibrary.Array_Add` (`self.graphActor`) _returnvalue_6))))))))

(event `DrawMap`
  ;[1 1 1] 미로 생성
  (goto _label))

(event `ResetMap`
  ;[1 1 1] 초기화
  (`|ExecutionSequence`
    (:`then_0`
      (bind _outactors (`GameplayStatics.GetAllActorsOfClass` "/Game/Search/BP_Points.BP_Points_C"))
      (`self.K2_DestroyActor` _outactors))
    (:`then_1`
      (set `self.IsFindEndPoint` false)
      (`KismetArrayLibrary.Array_Clear` (`self.arrCurrentCell`))
      (`KismetArrayLibrary.Array_Clear` (`self.graphActor`))
      (`self.DrawMap`))))

(event `SetCostVisibility`
  ;[1 1 1] Cost 활성화
  (for _array_element (`self.graphActor`)
    (`/Game/Search/BP_Points.SetCostVisibility` _array_element true)))

(event `StartDFS`
  (params (CurrentCell :type "/Game/Search/BP_Points Object Reference"))
  (bind _returnvalue (`KismetArrayLibrary.Array_Length` (`self.arrNeighborCell`)))
  (bind _output (`|GetArrayItem` (`self.arrCurrentCell`) (`KismetArrayLibrary.Array_LastIndex` (`self.arrCurrentCell`))))
  ;[1 1 1] DFS
  ;;[1 1 1] 기준이 되는 point 설정
  (`/Engine/EditorBlueprintResources/StandardMacros.IsValid` CurrentCell
    (:`Is Valid`
      (set `self.CurrentCell` CurrentCell))
    (:`Is Not Valid`
      (set `self.CurrentCell` (`self.StartPoint`))))
  (`KismetArrayLibrary.Array_Clear` (`self.arrNeighborCell`))
  ;;[1 1 1] CellArray에 End point 있는지 확인
  (`self.FindNeighborCell_Fuc`)
  (for _array_element (`self.arrNeighborCell`)
    (if (`/Game/Search/BP_Points.IsEndPoint` _array_element)
      (set `self.IsFindEndPoint` true)
      (else
        (`KismetArrayLibrary.Array_Add` (`self.arrCurrentCell`) _array_element))))
  ;;[1 1 1] 방문했던 Cell의 색상 변경
  (if (`self.IsFindEndPoint`)
    (for _array_element_2 (`self.arrCurrentCell`)
      (if (`/Game/Search/BP_Points.IsVisited` _array_element_2)
        (`/Game/Search/BP_Points.SetMaterial` _array_element_2 "/Game/Asset/Material/M_Base_Green.M_Base_Green")))
    (`self.DestinationReached`)
    (else
      ;;[1 1 1] 상하좌우 중 Cell이 있으면 랜덤으로 하나 정해서 Next Cell 설정 후 색상 변경
      ;; 만약 Cell 이 없으면 ArrCurrentCell 마지막 인덱스 -1 을 Next Cell 로 설정 후 함수 호출
      (if (== _returnvalue 0)
        (`KismetArrayLibrary.Array_Remove` (`self.arrCurrentCell`) (`KismetArrayLibrary.Array_LastIndex` (`self.arrCurrentCell`)))
        (`/Engine/EditorBlueprintResources/StandardMacros.IsValid` _output
          (:`Is Valid`
            (bind _output_get (set `self.NextCell` _output))
            (`/Game/Search/BP_Points.SetVisited` _output_get)
            (`self.StartDFS` (`self.NextCell`)))
          (:`Is Not Valid`
            (`self.DestinationUnreached`)))
        (else
          (bind _output_get_2 (set `self.NextCell` (`|GetArrayItem` (`self.arrNeighborCell`) (`KismetMathLibrary.RandomInteger` _returnvalue))))
          (`/Game/Search/BP_Points.SetVisited` _output_get_2)
          (`KismetSystemLibrary.Delay` 0.1)
          (`self.StartDFS` (`self.NextCell`)))))))

(event `StartDijkstra`
  (bind (_returnvalue_x _returnvalue_y) (`KismetMathLibrary.BreakVector` (`self.K2_GetActorLocation` (`self.CurrentCell`))))
  (bind (_returnvalue_x_2 _returnvalue_y_2) (`KismetMathLibrary.BreakVector` (`self.K2_GetActorLocation` (`self.CurrentCell`))))
  (bind (_returnvalue_x_3 _returnvalue_y_3) (`KismetMathLibrary.BreakVector` (`self.K2_GetActorLocation` (`self.CurrentCell`))))
  (bind (_returnvalue_x_4 _returnvalue_y_4) (`KismetMathLibrary.BreakVector` (`self.K2_GetActorLocation` (`self.CurrentCell`))))
  ;[1 1 1] Dijkstra
  ;;[1 1 1] 기준이 되는 point 설정
  (set `self.CurrentCell` (`self.StartPoint`))
  (`KismetArrayLibrary.Array_Clear` (`self.arrNeighborCell`))
  (`KismetArrayLibrary.Array_Add` (`self.arrCurrentCell`) (`self.CurrentCell`))
  (set `self.DijkstraCost` 0)
  (for _array_element (`self.arrCurrentCell`) :!label _label_2
    (set `self.CurrentCell` _array_element)
    (`self.FindNeighborCell_Dijkstra`))
  (if (`KismetArrayLibrary.Array_IsEmpty` (`self.arrNeighborCell`))
    ;;[1 1 1] EndPoint를 못찾았을 때
    (`KismetSystemLibrary.K2_ClearAndInvalidateTimerHandle` (`self.BFSTimer`))
    (`KismetArrayLibrary.Array_Clear` (`self.arrCurrentCell`))
    (`KismetArrayLibrary.Array_Clear` (`self.arrNeighborCell`))
    (`self.DestinationUnreached`)
    (else
      ;;[1 1 1] CellArray에 End point 있는지 확인
      (`/Engine/EditorBlueprintResources/StandardMacros.IncrementInt` (`self.DijkstraCost`)
        (:`  `
          (for _array_element_2 (`self.arrNeighborCell`)
            (if (`/Game/Search/BP_Points.IsEndPoint` _array_element_2)
              (set `self.IsFindEndPoint` true)
              (set `/Game/Search/BP_Points.Cost` (`self.DijkstraCost`) _array_element_2)
              (set `self.EndPoint` _array_element_2)
              (else
                (`/Game/Search/BP_Points.SetVisited` _array_element_2)
                (set `/Game/Search/BP_Points.Cost` (`self.DijkstraCost`) _array_element_2)
                (`KismetArrayLibrary.Array_Add` (`self.arrCurrentCell`) _array_element_2))))
          ;;[1 1 1] EndPoint 찾았는지 조건 확인
          (if (`self.IsFindEndPoint`)
            ;;[1 1 1] Start Point로 돌아가기
            (set `self.CurrentCell` (`self.EndPoint`))
            (for _array_element_3 (`self.graphActor`) :!label _label_3
              (if (not (`/Game/Search/BP_Points.IsWall` _array_element_3))
                (bind (_returnvalue_x_5 _returnvalue_y_5) (`KismetMathLibrary.BreakVector` (`self.K2_GetActorLocation` _array_element_3)))
                ;;;[1 1 1] 왼쪽 확인
                (if (and (== _returnvalue_x_5 (- _returnvalue_x_2 100.0)) (== _returnvalue_y_5 _returnvalue_y_2))
                  (`KismetArrayLibrary.Array_Add` (`self.arrNeighborCell`) _array_element_3))
                (bind (_returnvalue_x_6 _returnvalue_y_6) (`KismetMathLibrary.BreakVector` (`self.K2_GetActorLocation` _array_element_3)))
                ;;;[1 1 1] 오른쪽 확인
                (if (and (== _returnvalue_x_6 (+ _returnvalue_x_3 100.0)) (== _returnvalue_y_6 _returnvalue_y_3))
                  (`KismetArrayLibrary.Array_Add` (`self.arrNeighborCell`) _array_element_3))
                (bind (_returnvalue_x_7 _returnvalue_y_7) (`KismetMathLibrary.BreakVector` (`self.K2_GetActorLocation` _array_element_3)))
                ;;;[1 1 1] 위쪽 확인
                (if (and (== _returnvalue_y_7 (+ _returnvalue_y_4 100.0)) (== _returnvalue_x_7 _returnvalue_x_4))
                  (`KismetArrayLibrary.Array_Add` (`self.arrNeighborCell`) _array_element_3))
                (bind (_returnvalue_x_8 _returnvalue_y_8) (`KismetMathLibrary.BreakVector` (`self.K2_GetActorLocation` _array_element_3)))
                ;;;[1 1 1] 위쪽 확인
                (if (and (== _returnvalue_y_8 (- _returnvalue_y 100.0)) (== _returnvalue_x_8 _returnvalue_x))
                  (`KismetArrayLibrary.Array_Add` (`self.arrNeighborCell`) _array_element_3))))
            (for _array_element_4 (`self.arrNeighborCell`)
              (if (== (`/Game/Search/BP_Points.Cost` _array_element_4) (- (`self.DijkstraCost`) 1))
                (set `self.CurrentCell` _array_element_4)))
            (if (== (`self.DijkstraCost`) 1)
              (`KismetArrayLibrary.Array_Clear` (`self.arrCurrentCell`))
              (`KismetArrayLibrary.Array_Clear` (`self.arrNeighborCell`))
              (`self.DestinationReached`)
              (else
                (`/Engine/EditorBlueprintResources/StandardMacros.DecrementInt` (`self.DijkstraCost`)
                  (:`  `
                    (`KismetArrayLibrary.Array_Clear` (`self.arrNeighborCell`))
                    (`/Game/Search/BP_Points.SetMaterial` (`self.CurrentCell`) "/Game/Asset/Material/M_Base_Green.M_Base_Green")
                    (`self.FindNeighborCell_IngnoreVisit`)))))
            (else
              (`KismetArrayLibrary.Array_Clear` (`self.arrNeighborCell`))
              (`KismetSystemLibrary.Delay` 0.2)
              (`self.Research`))))))))

(event `Research`
  ;[1 1 1] Dijkstra
  (goto _label_2))

(event `ActivateVisitedCell`
  (bind _output (`|GetArrayItem` (`self.arrCurrentCell`) (- (`self.arrCurrentLengh`) 1)))
  ;[1 1 1] DFS
  ;;[1 0 0] 서서히 변하도록 타이머 사용 (미사용)
  (if (<= (`self.arrCurrentLengh`) 0)
    (`KismetSystemLibrary.K2_ClearAndInvalidateTimerHandle` (`self.DFSTimer`))
    (`self.DestinationReached`)
    (else
      (if (`/Game/Search/BP_Points.IsVisited` _output)
        (`/Game/Search/BP_Points.SetChangeColor` _output))
      (`/Engine/EditorBlueprintResources/StandardMacros.DecrementInt` (`self.arrCurrentLengh`)))))

(event `FindNeighborCell_IngnoreVisit`
  ;[1 1 1] Dijkstra
  ;;[1 1 1] Start Point로 돌아가기
  (goto _label_3))

(event `StartBFS`
  ;[1 1 1] BFS
  ;;[1 1 1] 기준이 되는 point 설정
  (set `self.CurrentCell` (`self.StartPoint`))
  (`KismetArrayLibrary.Array_Clear` (`self.arrNeighborCell`))
  (`KismetArrayLibrary.Array_Add` (`self.arrCurrentCell`) (`self.CurrentCell`))
  (bind _returnvalue (`KismetSystemLibrary.K2_SetTimerDelegate` (delegate `BFS`) 0.1 true))
  (set `self.BFSTimer` _returnvalue))

(event `BFS`
  ;[1 1 1] BFS
  (if (not (`KismetArrayLibrary.Array_IsEmpty` (`self.arrCurrentCell`)))
    (set `self.CurrentCell` (`|GetArrayItem` (`self.arrCurrentCell`)))
    (`KismetArrayLibrary.Array_Remove` (`self.arrCurrentCell`))
    (`self.FindNeighborCell_Fuc`)
    ;;[1 1 1] CellArray에 End point 있는지 확인
    (for _array_element (`self.arrNeighborCell`)
      (if (`/Game/Search/BP_Points.IsEndPoint` _array_element)
        (set `self.IsFindEndPoint` true)
        (else
          (`/Game/Search/BP_Points.SetVisited` _array_element)
          (`KismetArrayLibrary.Array_Add` (`self.arrCurrentCell`) _array_element)
          (`KismetArrayLibrary.Array_Add` (`self.arrTotalCell`) _array_element))))
    ;;[1 1 1] 방문했던 Cell의 색상 변경
    (if (`self.IsFindEndPoint`)
      (for _array_element_2 (`self.arrTotalCell`)
        (if (`/Game/Search/BP_Points.IsVisited` _array_element_2)
          (`/Game/Search/BP_Points.SetMaterial` _array_element_2 "/Game/Asset/Material/M_Base_Green.M_Base_Green")))
      (`KismetArrayLibrary.Array_Clear` (`self.arrTotalCell`))
      (`KismetSystemLibrary.K2_ClearAndInvalidateTimerHandle` (`self.BFSTimer`))
      (`self.DestinationReached`)
      (else
        (`KismetArrayLibrary.Array_Clear` (`self.arrNeighborCell`))))
    (else
      ;;[1 1 1] EndPoint를 못찾았을 때
      (`KismetSystemLibrary.K2_ClearAndInvalidateTimerHandle` (`self.BFSTimer`))
      (`KismetArrayLibrary.Array_Clear` (`self.arrTotalCell`))
      (`self.DestinationUnreached`))))

(fn `FindNeighborCell_Dijkstra`
  (bind (_returnvalue_x _returnvalue_y) (`KismetMathLibrary.BreakVector` (`self.K2_GetActorLocation` (`self.CurrentCell`))))
  (bind (_returnvalue_x_2 _returnvalue_y_2) (`KismetMathLibrary.BreakVector` (`self.K2_GetActorLocation` (`self.CurrentCell`))))
  (bind (_returnvalue_x_3 _returnvalue_y_3) (`KismetMathLibrary.BreakVector` (`self.K2_GetActorLocation` (`self.CurrentCell`))))
  (bind (_returnvalue_x_4 _returnvalue_y_4) (`KismetMathLibrary.BreakVector` (`self.K2_GetActorLocation` (`self.CurrentCell`))))
  ;[1 1 1] 근처 Cell 탐색
  (for _array_element (`self.graphActor`)
    (if (not (or (`/Game/Search/BP_Points.IsWall` _array_element) (`/Game/Search/BP_Points.IsVisited` _array_element)))
      (bind (_returnvalue_x_5 _returnvalue_y_5) (`KismetMathLibrary.BreakVector` (`self.K2_GetActorLocation` _array_element)))
      ;;[1 1 1] 왼쪽 확인
      (if (and (== _returnvalue_x_5 (- _returnvalue_x_2 100.0)) (== _returnvalue_y_5 _returnvalue_y_2))
        (set `/Game/Search/BP_Points.IsVisited` true _array_element)
        (`KismetArrayLibrary.Array_Add` (`self.arrNeighborCell`) _array_element))
      (bind (_returnvalue_x_6 _returnvalue_y_6) (`KismetMathLibrary.BreakVector` (`self.K2_GetActorLocation` _array_element)))
      ;;[1 1 1] 오른쪽 확인
      (if (and (== _returnvalue_x_6 (+ _returnvalue_x_3 100.0)) (== _returnvalue_y_6 _returnvalue_y_3))
        (set `/Game/Search/BP_Points.IsVisited` true _array_element)
        (`KismetArrayLibrary.Array_Add` (`self.arrNeighborCell`) _array_element))
      (bind (_returnvalue_x_7 _returnvalue_y_7) (`KismetMathLibrary.BreakVector` (`self.K2_GetActorLocation` _array_element)))
      ;;[1 1 1] 위쪽 확인
      (if (and (== _returnvalue_y_7 (+ _returnvalue_y_4 100.0)) (== _returnvalue_x_7 _returnvalue_x_4))
        (set `/Game/Search/BP_Points.IsVisited` true _array_element)
        (`KismetArrayLibrary.Array_Add` (`self.arrNeighborCell`) _array_element))
      (bind (_returnvalue_x_8 _returnvalue_y_8) (`KismetMathLibrary.BreakVector` (`self.K2_GetActorLocation` _array_element)))
      ;;[1 1 1] 위쪽 확인
      (if (and (== _returnvalue_y_8 (- _returnvalue_y 100.0)) (== _returnvalue_x_8 _returnvalue_x))
        (set `/Game/Search/BP_Points.IsVisited` true _array_element)
        (`KismetArrayLibrary.Array_Add` (`self.arrNeighborCell`) _array_element))))
  (return))

(fn `FindNeighborCell_Fuc`
  (bind (_returnvalue_x _returnvalue_y) (`KismetMathLibrary.BreakVector` (`self.K2_GetActorLocation` (`self.CurrentCell`))))
  (bind (_returnvalue_x_2 _returnvalue_y_2) (`KismetMathLibrary.BreakVector` (`self.K2_GetActorLocation` (`self.CurrentCell`))))
  (bind (_returnvalue_x_3 _returnvalue_y_3) (`KismetMathLibrary.BreakVector` (`self.K2_GetActorLocation` (`self.CurrentCell`))))
  (bind (_returnvalue_x_4 _returnvalue_y_4) (`KismetMathLibrary.BreakVector` (`self.K2_GetActorLocation` (`self.CurrentCell`))))
  ;[1 1 1] 근처 Cell 탐색
  (for _array_element (`self.graphActor`)
    (if (not (or (`/Game/Search/BP_Points.IsWall` _array_element) (`/Game/Search/BP_Points.IsVisited` _array_element)))
      (bind (_returnvalue_x_5 _returnvalue_y_5) (`KismetMathLibrary.BreakVector` (`self.K2_GetActorLocation` _array_element)))
      ;;[1 1 1] 왼쪽 확인
      (if (and (== _returnvalue_x_5 (- _returnvalue_x_2 100.0)) (== _returnvalue_y_5 _returnvalue_y_2))
        (`KismetArrayLibrary.Array_Add` (`self.arrNeighborCell`) _array_element))
      (bind (_returnvalue_x_6 _returnvalue_y_6) (`KismetMathLibrary.BreakVector` (`self.K2_GetActorLocation` _array_element)))
      ;;[1 1 1] 오른쪽 확인
      (if (and (== _returnvalue_x_6 (+ _returnvalue_x_3 100.0)) (== _returnvalue_y_6 _returnvalue_y_3))
        (`KismetArrayLibrary.Array_Add` (`self.arrNeighborCell`) _array_element))
      (bind (_returnvalue_x_7 _returnvalue_y_7) (`KismetMathLibrary.BreakVector` (`self.K2_GetActorLocation` _array_element)))
      ;;[1 1 1] 위쪽 확인
      (if (and (== _returnvalue_y_7 (+ _returnvalue_y_4 100.0)) (== _returnvalue_x_7 _returnvalue_x_4))
        (`KismetArrayLibrary.Array_Add` (`self.arrNeighborCell`) _array_element))
      (bind (_returnvalue_x_8 _returnvalue_y_8) (`KismetMathLibrary.BreakVector` (`self.K2_GetActorLocation` _array_element)))
      ;;[1 1 1] 위쪽 확인
      (if (and (== _returnvalue_y_8 (- _returnvalue_y 100.0)) (== _returnvalue_x_8 _returnvalue_x))
        (`KismetArrayLibrary.Array_Add` (`self.arrNeighborCell`) _array_element))))
  (return))

(fn `UserConstructionScript`)
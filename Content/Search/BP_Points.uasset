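; BP_Points is a cell actor that visualizes pathfinding search state for Dijkstra and A*.
; SetDijkstra and SetA* pick the mode and reveal a resized text label, which Tick refreshes with either Cost or scaled G and H values.
; SetVisited flags the cell and swaps its cube to a yellow material.
; SetChangeColor runs a timeline that fades the cube's Color parameter from yellow toward green.
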(event `self.ReceiveBeginPlay`
  (`self.SetCostVisibility` false))

(event `SetCostVisibility`
  (params (IsVisibility :type Boolean))
  ;[1 1 1] Text 활성화/비활성화
  (`SceneComponent.SetVisibility` (`self.T_Cost`) IsVisibility false))

(event `self.ReceiveTick`
  (params (DeltaSeconds :type "Float (single-precision)"))
  ;[1 1 1] cost 값 텍스트에 적용
  (if (`self.IsA*`)
    (`TextRenderComponent.K2_SetText` (`self.T_Cost`) (`|FormatText` "G:{G} H:{H}" (/ (`self.G`) 100.0) (/ (`self.H`) 100.0)))
    (else
      (`TextRenderComponent.K2_SetText` (`self.T_Cost`) (`KismetTextLibrary.Conv_IntToText` (`self.Cost`))))))

(event `SetDijkstra`
  ;[1 1 1] Dijkstra 설정
  (set `self.IsA*` false)
  (`self.SetCostVisibility` true)
  (`TextRenderComponent.SetWorldSize` (`self.T_Cost`) 100.0))

(event `SetMaterial`
  (params (Matrial :type "MaterialInstance Object Reference"))
  ;[1 1 1] 메테리얼 변경
  (`PrimitiveComponent.SetMaterial` (`self.Cube`) 0 Matrial))

(event `SetVisited`
  ;[1 1 1] Cell 방문 처리
  (set `self.IsVisited` true)
  (`self.SetMaterial` "/Game/Asset/Material/M_Base_Yellow.M_Base_Yellow"))

(event `SetA*`
  ;[1 1 1] A* 설정
  (set `self.IsA*` true)
  (`self.SetCostVisibility` true)
  (`TextRenderComponent.SetWorldSize` (`self.T_Cost`) 50.0))

(event `SetChangeColor`
  ;[1 1 1] 색상 변경
  (bind (_direction _newtrack_0) (`Timeline|Timeline`)
    (:`Update`
      (`MeshComponent.SetVectorParameterValueOnMaterials` (`self.Cube`) "Color" (`KismetMathLibrary.MakeVector` (`KismetMathLibrary.Lerp` 1.0 0.0 _newtrack_0) 1.0)))))

(fn `UserConstructionScript`)
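; BP_BasicPawn is a simple player-controlled pawn that flies freely with input axes for movement and look.
; MoveForward, MoveRight and MoveUp offset the actor along its local axes, scaled by MoveSpeed and frame delta time.
; Turn and LookUp feed controller yaw and pitch input, scaled by MouseSpeed and delta time.
; Movement uses direct local offsets rather than a movement component, and BeginPlay, Tick and the construction script are empty.
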(event `InputAxis|MoveForward`
  (params (AxisValue :type "Float (single-precision)"))
  (`self.K2_AddActorLocalOffset` (`KismetMathLibrary.MakeVector` (* AxisValue (`self.move_speed`) (`GameplayStatics.GetWorldDeltaSeconds`)))))

(event `InputAxis|Turn`
  (params (AxisValue :type "Float (single-precision)"))
  (`self.AddControllerYawInput` (* AxisValue (`self.mouse_speed`) (`GameplayStatics.GetWorldDeltaSeconds`))))

(event `InputAxis|LookUp`
  (params (AxisValue :type "Float (single-precision)"))
  (`self.AddControllerPitchInput` (* AxisValue (`self.mouse_speed`) (`GameplayStatics.GetWorldDeltaSeconds`))))

(event `InputAxis|MoveRight`
  (params (AxisValue :type "Float (single-precision)"))
  (`self.K2_AddActorLocalOffset` (`KismetMathLibrary.MakeVector` 0.0 (* AxisValue (`self.move_speed`) (`GameplayStatics.GetWorldDeltaSeconds`)))))

(event `InputAxis|MoveUp`
  (params (AxisValue :type "Float (single-precision)"))
  (`self.K2_AddActorLocalOffset` (`KismetMathLibrary.MakeVector` 0.0 0.0 (* AxisValue (`self.move_speed`) (`GameplayStatics.GetWorldDeltaSeconds`)))))

(fn `UserConstructionScript`)
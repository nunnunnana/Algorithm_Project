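; BP_SortActorMesh is an actor that builds a vertical stack of cube meshes, with its height driven by its Index value.
; On BeginPlay it loops up to Index, adding a movable cube StaticMeshComponent at runtime every 100 units along Z.
; SetActorColor recolors the whole stack by applying a given material to slot 0 of every StaticMeshComponent on the actor.
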(event `self.ReceiveBeginPlay`
  ;[1 1 1] index 값 만큼 메시 Spawn
  (for _index (range (+ (`self.Index`) 1))
    (`self.SpawnMesh` _index)))

(event `SpawnMesh`
  (params (Index :type Integer))
  ;[1 1 1] StaticmeshComponent의 mesh, mobility 설정
  (bind _returnvalue (`AddComponent|NODE_AddStaticMeshComponent-0` :`RelativeTransform` (`KismetMathLibrary.MakeTransform` (`KismetMathLibrary.MakeVector` 0.0 0.0 (`KismetMathLibrary.Conv_IntToDouble` (* Index 100))))))
  (bind _output_get (set `self.CurrentMesh` _returnvalue))
  (`SceneComponent.SetMobility` _output_get "Movable")
  (`StaticMeshComponent.SetStaticMesh` (`self.CurrentMesh`) "/Game/StarterContent/Shapes/Shape_Cube.Shape_Cube"))

(event `SetActorColor`
  (params (SetMaterial :type "MaterialInstance Object Reference"))
  ;[1 1 1] component의 색상 설정
  (for _array_element (`self.K2_GetComponentsByClass` "/Script/Engine.StaticMeshComponent")
    (`PrimitiveComponent.SetMaterial` _array_element 0 SetMaterial)))

(fn `UserConstructionScript`)
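; BP_SortActor is a visual selection sort demo built on a row of spawned BP_SortActorMesh actors, each storing its original Index.
; Z shuffles the array and X starts the sort, both ignored while sorting runs.
; A looping timer makes one comparison per tick, coloring the current minimum red, scanned elements blue or white and placed elements yellow.
; After each pass it swaps the minimum into place and realigns actor locations along Y to array order.
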(event `self.ReceiveBeginPlay`
  (`self.EnableInput` (`GameplayStatics.GetPlayerController` 0))
  (for _index (range (`self.Size`))
    (`self.CurrentCube`
      (:`then`
        (`self.SpawnCube` (`self.CurrentCube`) _index))
      (:`else`
        (`self.SpawnCube` self _index)))))

(event `MixedArray`
  ;[1 1 1] 액터 섞기
  (`KismetArrayLibrary.Array_Shuffle` (`self.arrTarget`))
  (`self.SetArrayLocation`))

(event `Key|Z`
  (params (Key :type "Key Structure"))
  ;[1 1 1] Input
  (:`Pressed`
    (if (not (`self.IsSorting`))
      (for (_ _array_index) (`self.arrTarget`)
        (`self.SetArrTargetColor` _array_index "/Game/Asset/Material/M_Base_White.M_Base_White"))
      (`self.MixedArray`))))

(event `SpawnCube`
  (params (Actor :type "Actor Object Reference") (Index :type Integer))
  (bind (_returnvalue_x _returnvalue_y _returnvalue_z) (`KismetMathLibrary.BreakVector` (`self.K2_GetActorLocation` Actor)))
  ;[1 1 1] Cube 액터 생성
  (bind _returnvalue (`|SpawnActorFromClass` "/Game/Sort/BP_SortActorMesh.BP_SortActorMesh_C" (`KismetMathLibrary.MakeTransform` (`KismetMathLibrary.MakeVector` _returnvalue_x (`KismetMathLibrary.Conv_IntToDouble` (* Index 100)) _returnvalue_z)) "Undefined" "MultiplyWithRoot" null null))
  (bind _output_get (set `self.CurrentCube` _returnvalue))
  (set `/Game/Sort/BP_SortActorMesh.Index` Index _output_get)
  (`KismetArrayLibrary.Array_Add` (`self.arrTarget`) (`self.CurrentCube`)))

(event `Key|X`
  (params (Key :type "Key Structure"))
  ;[1 1 1] Input
  (:`Pressed`
    (if (not (`self.IsSorting`))
      (for (_ _array_index) (`self.arrTarget`)
        (`self.SetArrTargetColor` _array_index "/Game/Asset/Material/M_Base_White.M_Base_White"))
      (`self.SelectionSort`))))

(event `Key|C`
  (params (Key :type "Key Structure"))
  ;[1 1 1] Input
)

(event `SetArrTargetColor`
  (params (index :type Integer) (SetMaterial :type "MaterialInstance Object Reference"))
  ;[1 1 1] 색상 선택
  (`/Game/Sort/BP_SortActorMesh.SetActorColor` (`|GetArrayItem` (`self.arrTarget`) index) SetMaterial))

(event `SetArrayLocation`
  ;[1 1 1] 배열의 인덱스 위치와 Location 값 동기화
  (for (_array_element _array_index) (`self.arrTarget`)
    (bind (_returnvalue_x _returnvalue_y _returnvalue_z) (`KismetMathLibrary.BreakVector` (`self.K2_GetActorLocation` _array_element)))
    (`self.K2_SetActorLocation` _array_element (`KismetMathLibrary.MakeVector` _returnvalue_x (`KismetMathLibrary.Conv_IntToDouble` (* _array_index 100)) _returnvalue_z) false false)))

(event `SelectionSort`
  ;[1 1 1] 선택정렬 실행
  (set `self.Index` 0)
  (`self.StartSelectionSort`)
  (set `self.IsSorting` true))

(event `StartSelectionSort`
  ;[1 1 1] 선택정렬 실행
  (if (> (`self.Index`) (- (`KismetArrayLibrary.Array_LastIndex` (`self.arrTarget`)) 1))
    (`self.SetArrTargetColor` (`self.Index`) "/Game/Asset/Material/M_Base_Yellow.M_Base_Yellow")
    (set `self.IsSorting` false)
    (else
      (bind _output_get (set `self.tmp` (`self.Index`)))
      (`self.SetArrTargetColor` _output_get "/Game/Asset/Material/M_Base_Red.M_Base_Red")
      (set `self.CurrentIndex` (+ (`self.Index`) 1))
      (bind _returnvalue (`KismetSystemLibrary.K2_SetTimerDelegate` (delegate `SetSelectionSortColor`) 0.01 true))
      (set `self.Timer` _returnvalue))))

(event `SetSelectionSortColor`
  (bind _returnvalue (- (`self.CurrentIndex`) 1))
  ;[1 1 1] 선택정렬 실행
  (if (not (== _returnvalue (`self.tmp`)))
    (`self.SetArrTargetColor` _returnvalue "/Game/Asset/Material/M_Base_White.M_Base_White"))
  (if (> (`self.CurrentIndex`) (`KismetArrayLibrary.Array_LastIndex` (`self.arrTarget`)))
    (`KismetSystemLibrary.K2_ClearAndInvalidateTimerHandle` (`self.Timer`))
    (`KismetArrayLibrary.Array_Swap` (`self.arrTarget`) (`self.Index`) (`self.tmp`))
    (`self.SetArrTargetColor` (`self.Index`) "/Game/Asset/Material/M_Base_Yellow.M_Base_Yellow")
    (`self.SetArrayLocation`)
    (`/Engine/EditorBlueprintResources/StandardMacros.IncrementInt` (`self.Index`)
      (:`  `
        (`self.StartSelectionSort`)))
    (else
      (if (>= (`/Game/Sort/BP_SortActorMesh.Index` (`|GetArrayItem` (`self.arrTarget`) (`self.tmp`))) (`/Game/Sort/BP_SortActorMesh.Index` (`|GetArrayItem` (`self.arrTarget`) (`self.CurrentIndex`))))
        (`self.SetArrTargetColor` (`self.tmp`) "/Game/Asset/Material/M_Base_White.M_Base_White")
        (bind _output_get (set `self.tmp` (`self.CurrentIndex`)))
        (`self.SetArrTargetColor` _output_get "/Game/Asset/Material/M_Base_Red.M_Base_Red")
        (else
          (`self.SetArrTargetColor` (`self.CurrentIndex`) "/Game/Asset/Material/M_Base_Blue.M_Base_Blue")))
      (`/Engine/EditorBlueprintResources/StandardMacros.IncrementInt` (`self.CurrentIndex`)))))

(fn `UserConstructionScript`)